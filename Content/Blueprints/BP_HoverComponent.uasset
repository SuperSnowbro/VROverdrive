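; Hover thruster scene component for BP_MegaCar that supplies an upward push based on its height above the surface below.
; Each tick it draws a debug line trace on the Visibility channel from its world location straight down by PropelDistance.
; On a hit, the normalized hit time is remapped through PowerScalingCurve to scale Power.
; The owning car receives that Z push along with the component reference through ReceiveHoverPush.
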(event EventTick
  (params (DeltaSeconds :type Float%20%28single-precision%29))
  (bind (_start _end) (CallFunction|GetLinetraceStartEnd))
  (bind (_outhit _returnvalue) (Collision|LineTraceByChannel _start _end "TraceTypeQuery1" false 0 "ForOneFrame"))
  (if _returnvalue
    (bind _asbp_mega_car (Utilities|Casting|CastToBP_MegaCar (Components|GetOwner)))
    (Default|ReceiveHoverPush _asbp_mega_car (Math|Vector|MakeVector 0.0 0.0 (Math|Float|Lerp 0.0 (Variables|Default|GetPower) (Math|Curves|GetFloatValue (Variables|Default|GetPowerScalingCurve) (.time _outhit)))) self)))

(event EventBeginPlay)

(fn GetLinetraceStartEnd
  (return (Transformation|GetWorldLocation) (- (Transformation|GetWorldLocation) (Math|Vector|MakeVector 0.0 0.0 (Variables|Default|GetPropelDistance)))))