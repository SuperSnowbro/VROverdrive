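; BP_MegaCar is a drivable physics hover vehicle with motion-controller interaction.
; Hover components supply push forces that are applied at their locations on the Physics body, while MoveForward and Turn axes add forward force and yaw torque.
; Either controller trigger runs a debug-drawn line trace from that controller and sends InteractMessage to the actor it hits.
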(event Custom|Receive%20Hover%20Push
  (params (Push :type Vector) (HoverComp :type Scene%20Component%20Object%20Reference))
  (Class|PrimitiveComponent|AddForceatLocation (Variables|Default|GetPhysics) Push (Transformation|GetWorldLocation HoverComp) "None"))

(event EventBeginPlay)

(event Collision|EventActorBeginOverlap
  (params (OtherActor :type Actor%20Object%20Reference)))

(event EventTick
  (params (DeltaSeconds :type Float%20%28single-precision%29)))

(event Input|AxisEvents|InputAxisMoveForward
  (params (AxisValue :type Float%20%28single-precision%29))
  (Physics|AddForce (Variables|Default|GetPhysics) (* (Math|Vector|GetForwardVector (Variables|Default|GetPhysics)) (* AxisValue (Variables|Default|GetSpeed))) "None" false))

(event Input|AxisEvents|InputAxisTurn
  (params (AxisValue :type Float%20%28single-precision%29))
  (Class|PrimitiveComponent|AddTorque (Variables|Default|GetPhysics) (Math|Vector|MakeVector 0.0 0.0 (* AxisValue (Variables|Default|GetTurnRate))) "None" true))

(event Custom|InteractRaycast
  (params (isRight :type Boolean))
  (bind _mcright (Variables|Default|GetMCRight))
  (bind _mcleft (Variables|Default|GetMCLeft))
  (bind _returnvalue (select isRight _mcright _mcleft))
  (bind _returnvalue_2 (Transformation|GetWorldLocation _returnvalue))
  (bind (_outhit _returnvalue_3) (Collision|LineTraceByChannel _returnvalue_2 (+ _returnvalue_2 (* (Math|Vector|GetForwardVector _returnvalue) (Variables|Default|GetInteractRange))) "TraceTypeQuery1" true 0 "ForDuration" true "(R=1.000000,G=0.000000,B=0.000000,A=1.000000)" "(R=0.000000,G=1.000000,B=0.000000,A=1.000000)" 2.0))
  (if _returnvalue_3
    (Class|BPIInteractable|Interact(Message) (.hitactor _outhit))))

(event Input|KeyboardEvents|MotionControllerRightTrigger
  (params (Key :type Key%20Structure :default "AnyKey"))
  (:Pressed
    (CallFunction|InteractRaycast true)))

(event Input|KeyboardEvents|MotionControllerLeftTrigger
  (params (Key :type Key%20Structure :default "AnyKey"))
  (:Pressed
    (CallFunction|InteractRaycast false)))

(fn ConstructionScript)